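; BP_AIPawn is a reinforcement-learning agent pawn that learns to move around without hitting obstacles, with game speed raised at BeginPlay.
; A movement actuator turns actions into forward input and yaw.
; Three line traces (left, center, right) supply normalized distances as observations.
; Step rewards survival, penalizes and terminates on near obstacles, and truncates at a step limit; Reset restores the start transform.
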(event `self.ReceiveBeginPlay`
  (set `self.StartTransform` (`self.GetTransform`))
  (`KismetSystemLibrary.ExecuteConsoleCommand` "slomo 5" null))

(event `self.ReceiveTick`
  (params (DeltaSeconds :type "Float (single-precision)")))

(event `self.MovementInputActuator.OnMovementDelegate`
  (params (MovementInput :type "Vector Structure (by ref)"))
  (`self.AddMovementInput` (`self.GetActorForwardVector`) MovementInput_X)
  (`self.K2_AddActorLocalRotation` (`KismetMathLibrary.MakeRotator` 0.0 0.0 (* MovementInput_Y 3.0))))

(fn `CollectObservations`
  (returns (OutObservations :type "InstancedStruct Structure"))
  (bind _returnvalue (`BlueprintInstancedStructLibrary.MakeInstancedStruct` (make `BoxPoint` (`|MakeArray` (/ (`self.DistLeft`) 1500.0) (/ (`self.DistCenter`) 2000.0) (/ (`self.DistRight`) 1500.0) :!type "Float (single-precision)") (`|MakeArray` 3))))
  (return _returnvalue))

(fn `GetObservationSpace`
  (returns (OutObservationSpace :type "InstancedStruct Structure"))
  (bind _returnvalue (`BlueprintInstancedStructLibrary.MakeInstancedStruct` (make `BoxSpace` (`|MakeArray` (make `BoxSpaceDimension` 0.0) (make `BoxSpaceDimension` 0.0) (make `BoxSpaceDimension` 0.0)) (`|MakeArray` 3))))
  (return _returnvalue))

(fn `InitializeEnvironment`
  (returns (OutAgentDefinition :type "InteractionDefinition Structure"))
  (set `self.StartTransform` (struct))
  (return (make `InteractionDefinition` "" (`ScholaSensor.GetObservationSpace`) (`ScholaActuator.GetActionSpace` (`self.MovementInputActuator`)))))

(fn `Reset`
  (returns (OutAgentState :type "InitialAgentState Structure"))
  (`self.K2_SetActorTransform` (`self.StartTransform`) false true)
  (`MovementComponent.StopMovementImmediately` (`self.FloatingPawnMovement`))
  (set `self.DistCenter` 2000.0)
  (set `self.DistLeft` 1500.0)
  (set `self.DistRight` 1500.0)
  (set `self.StepCount` 0)
  (`self.UpdateRaycasts`)
  (bind _outobservations (`ScholaSensor.CollectObservations`))
  (return (make `InitialAgentState` _outobservations)))

(fn `Step`
  (params (InAction :type "InstancedStruct Structure (by ref)"))
  (returns (OutAgentState :type "AgentState Structure"))
  (bind _returnvalue (or (< (`self.DistCenter`) 60.0) (< (`self.DistLeft`) 45.0) (< (`self.DistRight`) 45.0)))
  (`ScholaActuator.TakeAction` (`self.MovementInputActuator`) InAction)
  (`self.UpdateRaycasts`)
  (bind _output_get (set `self.StepCount` (+ (stale _output_get) 1)))
  (bind _outobservations (`ScholaSensor.CollectObservations`))
  (return (make `AgentState` (`KismetMathLibrary.SelectFloat` -10.0 0.1 _returnvalue) _returnvalue (>= _output_get 1500) _outobservations)))

(fn `UpdateRaycasts`
  (bind _raycenter (`self.RayCenter`))
  (bind _rayleft (`self.RayLeft`))
  (bind _rayright (`self.RayRight`))
  (bind _returnvalue (`SceneComponent.K2_GetComponentLocation` _raycenter))
  (bind _returnvalue_2 (`SceneComponent.K2_GetComponentLocation` _rayleft))
  (bind _returnvalue_3 (`SceneComponent.K2_GetComponentLocation` _rayright))
  (`|ExecutionSequence`
    (:`then_0`
      (bind (_outhit _returnvalue_4) (`KismetSystemLibrary.LineTraceSingle` :`Start` _returnvalue :`End` (+ (* (`SceneComponent.GetForwardVector` _raycenter) 2000.0) _returnvalue) :`TraceChannel` "TraceTypeQuery1" :`DrawDebugType` "ForOneFrame"))
      (set `self.DistCenter` (`KismetMathLibrary.SelectFloat` (`.Distance` (`GameplayStatics.BreakHitResult` _outhit)) 2000.0 _returnvalue_4)))
    (:`then_1`
      (bind (_outhit_2 _returnvalue_5) (`KismetSystemLibrary.LineTraceSingle` :`Start` _returnvalue_2 :`End` (+ (* (`SceneComponent.GetForwardVector` _rayleft) 1500.0) _returnvalue_2) :`TraceChannel` "TraceTypeQuery1" :`DrawDebugType` "ForOneFrame"))
      (set `self.DistLeft` (`KismetMathLibrary.SelectFloat` (`.Distance` (`GameplayStatics.BreakHitResult` _outhit_2)) 1500.0 _returnvalue_5)))
    (:`then_2`
      (bind (_outhit_3 _returnvalue_6) (`KismetSystemLibrary.LineTraceSingle` :`Start` _returnvalue_3 :`End` (+ (* (`SceneComponent.GetForwardVector` _rayright) 1500.0) _returnvalue_3) :`TraceChannel` "TraceTypeQuery1" :`DrawDebugType` "ForOneFrame"))
      (set `self.DistRight` (`KismetMathLibrary.SelectFloat` (`.Distance` (`GameplayStatics.BreakHitResult` _outhit_3)) 1500.0 _returnvalue_6)))))

(fn `UserConstructionScript`)